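; Cannon actor that automatically fires projectiles on a repeating timer from BeginPlay.
; After each reload delay it spawns the configured projectile class at the Arrow component's location and rotation, using a configurable scale.
; Each shot then triggers a timeline that animates the Cannon1 component along its relative Y axis as a firing motion.
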(event `self.ReceiveBeginPlay`
  (`KismetSystemLibrary.Delay` (`self.reload_duration`) :!label _label)
  (`self.Shoot_projectile`)
  (`self.cannon fired`)
  (goto _label))

(event `cannon fired`
  (bind (_direction _newtrack_0) (`Timeline|Timeline_0` :!via `PlayFromStart`)
    (:`Update`
      (`SceneComponent.K2_SetRelativeLocation` (`self.Cannon1`) (`KismetMathLibrary.MakeVector` 0.0 _newtrack_0) false false))))

(fn `Shoot_projectile`
  (bind (_returnvalue_location _returnvalue_rotation) (`KismetMathLibrary.BreakTransform` (`SceneComponent.K2_GetComponentToWorld` (`self.Arrow`))))
  (`|SpawnActorFromClass` "/Game/Blueprint/actors/projectiles/projectile.projectile_C" (`KismetMathLibrary.MakeTransform` _returnvalue_location _returnvalue_rotation (`KismetMathLibrary.Conv_DoubleToVector` (`self.projectile_scale`))) "Undefined" "OverrideRootScale" null null))

(fn `UserConstructionScript`)