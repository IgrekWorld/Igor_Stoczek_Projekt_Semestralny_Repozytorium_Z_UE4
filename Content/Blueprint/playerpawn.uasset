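; Player pawn that moves by applying torque to its static mesh and restarts the level when it takes any damage.
; Both input axes share one torque node, driving X and Y equally with acceleration change.
; Damage calls Umieranie (Polish for "dying"), which fades to black, then the current level reopens after the fade.
; BeginPlay starts a fade-in whose duration reads Umieranie's output without calling it.
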(event `self.ReceiveBeginPlay`
  (`PlayerCameraManager.StartCameraFade` :`self` (`GameplayStatics.GetPlayerCameraManager` 0) :`FromAlpha` 1.0 :`Duration` (stale `self.ReceiveAnyDamage` _returnvalue)))

(event `self.ReceiveAnyDamage`
  (params (Damage :type "Float (single-precision)") (DamageType :type "DamageType Object Reference") (InstigatedBy :type "Controller Object Reference") (DamageCauser :type "Actor Object Reference"))
  (bind (_returnvalue _returnvalue2) (`self.Umieranie` (`GameplayStatics.GetPlayerCameraManager` 0)))
  (`KismetSystemLibrary.Delay` _returnvalue)
  (`GameplayStatics.OpenLevel` (`KismetStringLibrary.Conv_StringToName` _returnvalue2)))

(event `InputAxis|ForwardBackwards`
  (params (AxisValue :type "Float (single-precision)"))
  (bind _newvar_0 (`self.NewVar_0`))
  (`PrimitiveComponent.AddTorqueInRadians` (`self.StaticMesh`) (`KismetMathLibrary.MakeVector` (* (stale `InputAxis|LeftRight` AxisValue) _newvar_0) (* AxisValue _newvar_0)) "None" true :!label _label))

(event `InputAxis|LeftRight`
  (params (AxisValue :type "Float (single-precision)"))
  (goto _label))

(fn `Umieranie`
  (params (self2 :type "PlayerCameraManager Object Reference"))
  (returns (ReturnValue :type "Float (double-precision)") (ReturnValue2 :type String))
  (`PlayerCameraManager.StartCameraFade` :`self` self2 :`ToAlpha` 1.0 :`Duration` 3.0)
  (bind _returnvalue (`GameplayStatics.GetCurrentLevelName` true))
  (return 3.0 _returnvalue))

(fn `UserConstructionScript`)